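; BP_personaje is a player-controllable character Blueprint that handles basic walking and camera-look input.
; The Caminaadelante and Caminaderecha axes add movement along forward and right vectors built from the control rotation's yaw only, so look pitch does not affect movement direction.
; The miralado and miraarriba axes feed controller yaw and pitch directly.
; BeginPlay, Tick, overlap and the construction script are empty.
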(event EventBeginPlay)

(event Collision|EventActorBeginOverlap
  (params (OtherActor :type Actor%20Object%20Reference)))

(event EventTick
  (params (DeltaSeconds :type Float%20%28single-precision%29)))

(event Input|AxisEvents|InputAxisCaminaadelante
  (params (AxisValue :type Float%20%28single-precision%29))
  ;[1 1 1] Movimiento
  (Pawn|Input|AddMovementInput (Math|Vector|GetForwardVector (Math|Rotator|MakeRotator 0.0 0.0 (.Yaw (Math|Rotator|BreakRotator (Pawn|GetControlRotation :!class /Script/Engine.Pawn))))) AxisValue false))

(event Input|AxisEvents|InputAxisCaminaderecha
  (params (AxisValue :type Float%20%28single-precision%29))
  ;[1 1 1] Movimiento
  (Pawn|Input|AddMovementInput (Math|Vector|GetRightVector (Math|Rotator|MakeRotator 0.0 0.0 (.Yaw (Math|Rotator|BreakRotator (Pawn|GetControlRotation :!class /Script/Engine.Pawn))))) AxisValue false))

(event Input|AxisEvents|InputAxismiralado
  (params (AxisValue :type Float%20%28single-precision%29))
  ;[1 1 1] ComplementoMovimiento
  (Pawn|Input|AddControllerYawInput AxisValue))

(event Input|AxisEvents|InputAxismiraarriba
  (params (AxisValue :type Float%20%28single-precision%29))
  ;[1 1 1] ComplementoMovimiento
  (Pawn|Input|AddControllerPitchInput AxisValue))

(fn ConstructionScript)